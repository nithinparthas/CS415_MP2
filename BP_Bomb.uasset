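; BP_Bomb is a projectile that swells like a blast and destroys itself after overlapping any actor other than BP_Mortar.
; The overlap sets an Expansion flag, and Tick then stops ProjectileMovement and grows the actor by a fixed, frame-rate-dependent step until it reaches a size limit.
; A player damage chain with health bar update and restart display is present but disconnected, so it never runs.
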(event `self.ReceiveActorBeginOverlap`
  (params (OtherActor :type "Actor Object Reference"))
  (cast `/Game/LearningKit_Games/Blueprints/PlayerCharacter/BP_Mortar` OtherActor
    (:`CastFailed`
      (set `self.Expansion` true))))

(event `self.ReceiveTick`
  (params (DeltaSeconds :type "Float (single-precision)"))
  (if (`self.Expansion`)
    (`MovementComponent.StopMovementImmediately` (`self.ProjectileMovement`))
    (`self.SetActorScale3D` (+ (`self.GetActorScale3D`) (0.2 0.2 0.2)))
    (if (>= (`KismetMathLibrary.GetMaxElement` (`self.GetActorScale3D`)) 4.0)
      (set `self.Expansion` false)
      (`self.SetActorScale3D` (1.0 1.0 1.0))
      (`self.K2_DestroyActor`))))

(fn `UserConstructionScript`)