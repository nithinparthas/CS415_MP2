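; BP_Disruptor is a hazard that shoots at the player, disrupts their movement up close, and is destroyed on Box overlap.
; A looping timer spawns BP_Pellet projectiles aimed at the player.
; Tick polls overlaps: Box destroys the actor, otherwise Sphere damages and lifts the player, blocks input and movement, and applies a horizontal launch toward the disruptor.
; A short Delay then restores game input and walking.
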(event `self.ReceiveTick`
  (params (DeltaSeconds :type "Float (single-precision)"))
  (bind _asbp_learning_kit_player_character (cast `/Game/LearningKit_Games/Blueprints/PlayerCharacter/BP_LearningKit_PlayerCharacter` (`GameplayStatics.GetPlayerPawn` 0)))
  (if (`PrimitiveComponent.IsOverlappingActor` (`self.Box`) _asbp_learning_kit_player_character)
    (`self.K2_DestroyActor`)
    (elif (`PrimitiveComponent.IsOverlappingActor` (`self.Sphere`) _asbp_learning_kit_player_character)
      (`/Game/LearningKit_Games/Blueprints/PlayerCharacter/BP_LearningKit_PlayerCharacter.TakeDamage` _asbp_learning_kit_player_character 15.0)
      (bind _returnvalue (`self.K2_GetActorLocation` _asbp_learning_kit_player_character))
      (`self.K2_TeleportTo` :`self` _asbp_learning_kit_player_character :`DestLocation` (+ _returnvalue (0.0 0.0 100.0)))
      (`WidgetBlueprintLibrary.SetInputMode_UIOnlyEx` (`GameplayStatics.GetPlayerController` 0) null)
      (bind _charactermovement (`Character.CharacterMovement` _asbp_learning_kit_player_character))
      (`CharacterMovementComponent.DisableMovement` _charactermovement)
      (`MovementComponent.StopMovementImmediately` _charactermovement)
      (`Character.LaunchCharacter` _asbp_learning_kit_player_character (* (`KismetMathLibrary.GetDirectionUnitVector` (`self.K2_GetActorLocation`) _returnvalue) (-350.0 -350.0 0.0)) false false)
      (`KismetSystemLibrary.Delay` 0.5)
      (`WidgetBlueprintLibrary.SetInputMode_GameOnly` (`GameplayStatics.GetPlayerController` 0))
      (`CharacterMovementComponent.SetMovementMode` _charactermovement "MOVE_Walking" 0))))

(event `self.ReceiveBeginPlay`
  (`KismetSystemLibrary.K2_SetTimerDelegate` (delegate `Activate`) 1.0 true))

(event `Activate`
  (bind _velocity (`self.Velocity`))
  (bind _returnvalue (`|SpawnActorFromClass` "/Game/LearningKit_Games/Blueprints/PlayerCharacter/BP_Pellet.BP_Pellet_C" (`self.GetTransform`) "Undefined" "MultiplyWithRoot" null null))
  (bind _asbp_learning_kit_player_character (cast `/Game/LearningKit_Games/Blueprints/PlayerCharacter/BP_LearningKit_PlayerCharacter` (`GameplayStatics.GetPlayerPawn` 0)))
  (`ProjectileMovementComponent.SetVelocityInLocalSpace` (`/Game/LearningKit_Games/Blueprints/PlayerCharacter/BP_Pellet.ProjectileMovement` _returnvalue) (* (`KismetMathLibrary.GetDirectionUnitVector` (`self.K2_GetActorLocation`) (`self.K2_GetActorLocation` _asbp_learning_kit_player_character)) (`KismetMathLibrary.MakeVector` _velocity _velocity _velocity))))

(fn `UserConstructionScript`)