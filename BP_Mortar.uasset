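; BP_Mortar is a hazard actor that lobs BP_Bomb projectiles in random, upward-biased directions until the player reaches it.
; A looping timer fires Activate, which spawns a bomb and sets its local projectile velocity from the Velocity variable, random per-axis factors and an upward offset.
; Tick polls whether the learning-kit player overlaps Box and destroys the mortar if so.
; Disconnected nodes for score-based velocity scaling never run.
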(event `self.ReceiveBeginPlay`
  (`KismetSystemLibrary.K2_SetTimerDelegate` (delegate `Activate`) 2.0 true))

(event `Activate`
  (bind _velocity (`self.Velocity`))
  (bind _returnvalue (`|SpawnActorFromClass` "/Game/LearningKit_Games/Blueprints/PlayerCharacter/BP_Bomb.BP_Bomb_C" (`self.GetTransform`) "Undefined" "MultiplyWithRoot" null null))
  (`ProjectileMovementComponent.SetVelocityInLocalSpace` (`/Game/LearningKit_Games/Blueprints/PlayerCharacter/BP_Bomb.ProjectileMovement` _returnvalue) (+ (* (`KismetMathLibrary.MakeVector` _velocity _velocity _velocity) (`KismetMathLibrary.MakeVector` (`KismetMathLibrary.RandomFloatInRange` -2.5 2.5) (`KismetMathLibrary.RandomFloatInRange` -2.5 2.5) (`KismetMathLibrary.RandomFloatInRange` 0.0 2.5))) (0.0 0.0 200.0))))

(event `self.ReceiveTick`
  (params (DeltaSeconds :type "Float (single-precision)"))
  (bind _asbp_learning_kit_player_character (cast `/Game/LearningKit_Games/Blueprints/PlayerCharacter/BP_LearningKit_PlayerCharacter` (`GameplayStatics.GetPlayerPawn` 0)))
  (if (`PrimitiveComponent.IsOverlappingActor` (`self.Box`) _asbp_learning_kit_player_character)
    (`self.K2_DestroyActor`)))

(fn `UserConstructionScript`)