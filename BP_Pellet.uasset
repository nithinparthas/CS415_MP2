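; BP_Pellet is a pellet actor that destroys itself when it overlaps any actor other than a BP_Disruptor.
; The overlap event holds the only active logic, with Tick, BeginPlay and the construction script left empty.
; An unconnected chain that never runs would damage the LearningKit player character, update its health bar and show a restart prompt on death.
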(event `self.ReceiveActorBeginOverlap`
  (params (OtherActor :type "Actor Object Reference"))
  (cast `/Game/LearningKit_Games/Blueprints/PlayerCharacter/BP_Disruptor` OtherActor
    (:`CastFailed`
      (`self.K2_DestroyActor`))))

(event `self.ReceiveBeginPlay`)

(fn `UserConstructionScript`)